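; BP_Enemy_Base is a base enemy actor that moves in straight lines between direction updates on a 100-unit grid.
; A looping 0.01-second timer, capped at once per frame, calls Movement to add direction times speed without sweep or delta-time scaling.
; The UpdateDirection event stores a new direction and snaps the actor to the given grid point.
; Both paths swap X and Y when converting to world space.
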(event `self.ReceiveBeginPlay`
  (`KismetSystemLibrary.K2_SetTimer` null "Movement" 0.01 true true))

(event `/Game/Interface/BPI_Enemies.UpdateDirection`
  (params (Direction :type "IntPoint Structure") (CurPoint :type "IntPoint Structure"))
  (bind (_x _y) (break `IntPoint` CurPoint))
  (set `self.MovementDirection` Direction)
  (`self.K2_SetActorLocation` (`KismetMathLibrary.MakeVector` (* _y 100.0) (* _x 100.0))))

(fn `Movement`
  (bind (_movementdirection_x _movementdirection_y) (break `IntPoint` (`self.MovementDirection`)))
  (`self.K2_SetActorLocation` (+ (`self.K2_GetActorLocation`) (`KismetMathLibrary.MakeVector` (* _movementdirection_y (`self.MovementSpeed`)) (* _movementdirection_x (`self.MovementSpeed`))))))

(fn `UserConstructionScript`)