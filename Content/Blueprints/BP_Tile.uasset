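; BP_Tile is a grid tile that highlights under the cursor and directs enemies along a path.
; Hovering reports its Coord to the player pawn, and leaving restores the material matching its State (Empty, Blocked, Path, Start or End).
; Its box overlap passes the tile's Direction and Coord to BPI_Enemies actors through interface messages.
; End tiles also send those actors massive damage flagged as end-box.
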(event `self.Plane.OnBeginCursorOver`
  (params (TouchedComponent :type "PrimitiveComponent Object Reference"))
  (`/Engine/EditorBlueprintResources/StandardMacros.DoOnce` false :!label _label
    (:`Completed`
      (message `/Game/Interface/BPI_Towers.SetHoveredTile` (`GameplayStatics.GetPlayerPawn` 0) (`self.Coord`))
      (`PrimitiveComponent.SetMaterial` (`self.Plane`) 0 "/Game/Material/MI_Highlight.MI_Highlight"))))

(event `self.Plane.OnEndCursorOver`
  (params (TouchedComponent :type "PrimitiveComponent Object Reference"))
  (`|ExecutionSequence`
    (:`then_0`
      (goto _label :!via `Reset`))
    (:`then_1`
      (`self.ColourReset`))))

(event `self.Box.OnComponentBeginOverlap`
  (params (OverlappedComponent :type "PrimitiveComponent Object Reference") (OtherActor :type "Actor Object Reference") (OtherComp :type "PrimitiveComponent Object Reference") (OtherBodyIndex :type Integer) (bFromSweep :type Boolean) (SweepResult :type "HitResult Structure (by ref)"))
  (if (`KismetSystemLibrary.DoesImplementInterface` OtherActor "/Game/Interface/BPI_Enemies.BPI_Enemies_C")
    (message `/Game/Interface/BPI_Enemies.UpdateDirection` OtherActor (`self.Direction`) (`self.Coord`))
    (if (`|EnumEquality` (`self.State`) "NewEnumerator4")
      (message `/Game/Interface/BPI_Enemies.Damage` OtherActor 99999.0 true))))

(event `/Game/Interface/BPI_Enemies.UpdateDirection`
  (params (Direction :type "IntPoint Structure") (CurPoint :type "IntPoint Structure"))
  (set `self.Direction` Direction))

(fn `ColourReset`
  (switch `/Game/DATA/ETileStates` (`self.State`)
    (:`NewEnumerator0`
      (set `self.DefaultMat` "/Game/Material/MI_White.MI_White"))
    (:`NewEnumerator1`
      (set `self.DefaultMat` "/Game/Material/MI_Blocked.MI_Blocked"))
    (:`NewEnumerator2`
      (set `self.DefaultMat` "/Game/Material/MI_DebugBlue.MI_DebugBlue"))
    (:`NewEnumerator3`
      (set `self.DefaultMat` "/Game/Material/MI_Gren.MI_Gren"))
    (:`NewEnumerator4`
      (set `self.DefaultMat` "/Game/Material/MI_Red.MI_Red")))
  (`self.SetColour`))

(fn `SetColour`
  (`PrimitiveComponent.SetMaterial` (`self.Plane`) 0 (`self.DefaultMat`)))

(fn `UserConstructionScript`)