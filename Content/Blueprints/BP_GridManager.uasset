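; Grid manager for a tower defense game that spawns the tile grid, marks start and end, and lifts the player pawn above it.
; PlaceTower spawns a tower if TryPlaceTower allows, then reruns FindPath, sends each path tile its direction, recolours tiles and spawns an enemy near the start, even if placement failed.
; TempPath previews the route from TempPlaceTower without spawning.
; Placement checks and pathfinding are defined outside these graphs.
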(event `self.ReceiveBeginPlay`
  (bind (_end_x _end_y) (break `IntPoint` (`self.End`)))
  (bind (_start_x _start_y) (break `IntPoint` (`self.Start`)))
  (bind (_returnvalue_x _returnvalue_y) (`KismetMathLibrary.BreakVector` (`self.K2_GetActorLocation` (`|GetArrayItem` (`self.Tiles`) (/ (- (`KismetArrayLibrary.Array_Length` (`self.Tiles`)) 1) 2)))))
  ; y
  (for _index (range (`self.GridHeight`))
    ; x
    (for _index_2 (range (`self.GridWidth`))
      (bind _returnvalue (`|SpawnActorFromClass` "/Game/Blueprints/BP_Tile.BP_Tile_C" (`KismetMathLibrary.MakeTransform` (`KismetMathLibrary.MakeVector` (* _index 100.0) (* _index_2 100.0))) "AlwaysSpawn" "MultiplyWithRoot" null null))
      (`KismetArrayLibrary.Array_Add` (`self.Tiles`) _returnvalue)
      (set `/Game/Blueprints/BP_Tile.Coord` (make `IntPoint` _index_2 _index) _returnvalue)))
  (`KismetSystemLibrary.Delay` 1.0)
  (`PrimitiveComponent.SetMaterial` (`/Game/Blueprints/BP_Tile.Plane` (`|GetArrayItem` (`self.Tiles`) (+ _start_x (* _start_y (`self.GridWidth`))))) 0 "/Game/Material/MI_Gren.MI_Gren")
  (`PrimitiveComponent.SetMaterial` (`/Game/Blueprints/BP_Tile.Plane` (`|GetArrayItem` (`self.Tiles`) (+ _end_x (* _end_y (`self.GridWidth`))))) 0 "/Game/Material/MI_Red.MI_Red")
  (`self.K2_SetActorLocation` (`GameplayStatics.GetPlayerPawn` 0) (`KismetMathLibrary.MakeVector` _returnvalue_x _returnvalue_y 1500.0) false false))

(fn `Place Tower`
  (params (Coord :type "IntPoint Structure"))
  (bind (_x _y) (break `IntPoint` Coord))
  (bind (_start_x _start_y) (break `IntPoint` (`self.Start`)))
  (bind (_end_x _end_y) (break `IntPoint` (`self.End`)))
  (bind (_start_x_2 _start_y_2) (break `IntPoint` (`self.Start`)))
  (bind _output (`|GetArrayItem` (`self.Tiles`) (+ _x (* _y (`self.GridWidth`)))))
  (bind _returnvalue (`self.TryPlaceTower` Coord))
  (if _returnvalue
    (set `/Game/Blueprints/BP_Tile.State` "NewEnumerator1" _output)
    (`|SpawnActorFromClass` "/Game/Blueprints/BP_Tower_Base.BP_Tower_Base_C" (`KismetMathLibrary.MakeTransform` (+ (`self.K2_GetActorLocation` _output) (0.0 0.0 30.0))) "Undefined" "MultiplyWithRoot" null null)
    (`KismetArrayLibrary.Array_Add` (`self.Towers`) Coord))
  (for _array_element (`self.Tiles`)
    (if (`|EnumInequality` (`/Game/Blueprints/BP_Tile.State` _array_element) "NewEnumerator1")
      (set `/Game/Blueprints/BP_Tile.State` "NewEnumerator0" _array_element)))
  (bind _outpath (`self.FindPath`))
  (for (_array_element_2 _array_index) _outpath
    (if (not (== _array_index (- (`KismetArrayLibrary.Array_Length` _outpath) 1)))
      (bind (_x_2 _y_2) (break `IntPoint` (`|GetArrayItem` _outpath (+ _array_index 1))))
      (bind _intpoint (make `IntPoint` (- _x_2 (break `IntPoint` _array_element_2)) (- _y_2 (`.Y` (break `IntPoint` _array_element_2)))))
      (`KismetSystemLibrary.PrintString` (`KismetStringLibrary.Conv_IntPointToString` _intpoint))
      (message `/Game/Interface/BPI_Enemies.UpdateDirection` (`|GetArrayItem` (`self.Tiles`) (+ (break `IntPoint` _array_element_2) (* (`.Y` (break `IntPoint` _array_element_2)) (`self.GridWidth`)))) _intpoint (make `IntPoint` (break `IntPoint` _array_element_2) (`.Y` (break `IntPoint` _array_element_2)))))
    (set `/Game/Blueprints/BP_Tile.State` "NewEnumerator2" (`|GetArrayItem` (`self.Tiles`) (+ (break `IntPoint` _array_element_2) (* (`.Y` (break `IntPoint` _array_element_2)) (`self.GridWidth`))))))
  (for _array_element_3 (`self.Tiles`)
    (`/Game/Blueprints/BP_Tile.ColourReset` _array_element_3))
  (`PrimitiveComponent.SetMaterial` (`/Game/Blueprints/BP_Tile.Plane` (`|GetArrayItem` (`self.Tiles`) (+ _start_x_2 (* _start_y_2 (`self.GridWidth`))))) 0 "/Game/Material/MI_Gren.MI_Gren")
  (`PrimitiveComponent.SetMaterial` (`/Game/Blueprints/BP_Tile.Plane` (`|GetArrayItem` (`self.Tiles`) (+ _end_x (* _end_y (`self.GridWidth`))))) 0 "/Game/Material/MI_Red.MI_Red")
  (`|SpawnActorFromClass` "/Game/Blueprints/BP_Enemy_Base.BP_Enemy_Base_C" (`KismetMathLibrary.MakeTransform` (- (`self.K2_GetActorLocation` (`|GetArrayItem` (`self.Tiles`) (+ _start_x (* _start_y (`self.GridWidth`))))) (0.0 50.0 0.0))) "Undefined" "MultiplyWithRoot" null null))

(fn `Temp Path`
  (params (Pos :type "IntPoint Structure"))
  (bind (_end_x _end_y) (break `IntPoint` (`self.End`)))
  (bind (_start_x _start_y) (break `IntPoint` (`self.Start`)))
  (bind (_outpath _returnvalue) (`self.TempPlaceTower` Pos))
  (if _returnvalue
    (for _array_element (`self.Tiles`)
      (if (`|EnumInequality` (`/Game/Blueprints/BP_Tile.State` _array_element) "NewEnumerator1")
        (set `/Game/Blueprints/BP_Tile.State` "NewEnumerator0" _array_element)))
    (for _array_element_2 _outpath
      (set `/Game/Blueprints/BP_Tile.State` "NewEnumerator2" (`|GetArrayItem` (`self.Tiles`) (+ (break `IntPoint` _array_element_2) (* (`.Y` (break `IntPoint` _array_element_2)) (`self.GridWidth`))))))
    (for _array_element_3 (`self.Tiles`)
      (`/Game/Blueprints/BP_Tile.ColourReset` _array_element_3))
    (`PrimitiveComponent.SetMaterial` (`/Game/Blueprints/BP_Tile.Plane` (`|GetArrayItem` (`self.Tiles`) (+ _start_x (* _start_y (`self.GridWidth`))))) 0 "/Game/Material/MI_Gren.MI_Gren")
    (`PrimitiveComponent.SetMaterial` (`/Game/Blueprints/BP_Tile.Plane` (`|GetArrayItem` (`self.Tiles`) (+ _end_x (* _end_y (`self.GridWidth`))))) 0 "/Game/Material/MI_Red.MI_Red")))

(fn `UserConstructionScript`)