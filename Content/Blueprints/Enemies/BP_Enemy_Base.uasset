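; Base enemy that moves along grid directions and dies on reaching the end box or at zero HP.
; A looping timer steps its location, while UpdateDirection snaps it to grid points with X and Y swapped.
; The player UI's 2X event doubles or restores speed.
; Damage sets HP to clamped Amount minus HP; deaths notify BP_GridManager, and the resource update is only a print.
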(event `self.ReceiveBeginPlay`
  (`KismetSystemLibrary.K2_SetTimer` null "Movement" 0.01 true true)
  (bind _asbp_player (cast `/Game/Blueprints/BP_Player` (`GameplayStatics.GetPlayerPawn` 0)))
  (add `/Game/UI/WBP_Tower.2XSpeed` (`/Game/Blueprints/BP_Player.Main UI` _asbp_player) (delegate `Speed Set`))
  (set `self.Defualt Move Speed` (`self.MovementSpeed`)))

(event `Speed Set`
  (params (is2X :type Boolean))
  (if is2X
    (set `self.MovementSpeed` (* (`self.MovementSpeed`) 2.0))
    (else
      (set `self.MovementSpeed` (`self.Defualt Move Speed`)))))

(event `/Game/Interface/BPI_Enemies.UpdateDirection`
  (params (Direction :type "IntPoint Structure") (CurPoint :type "IntPoint Structure"))
  (bind (_x _y) (break `IntPoint` CurPoint))
  (set `self.MovementDirection` Direction)
  (`self.K2_SetActorLocation` (`KismetMathLibrary.MakeVector` (* _y 100.0) (* _x 100.0))))

(event `/Game/Interface/BPI_Enemies.Damage`
  (params (Amount :type "Float (double-precision)") (isEndBox :type Boolean))
  (if isEndBox
    (bind _returnvalue (`GameplayStatics.GetActorOfClass` "/Game/Blueprints/BP_GridManager.BP_GridManager_C"))
    (message `/Game/Interface/BPI_Grid.DeadEnemy` _returnvalue)
    (`self.K2_DestroyActor`)
    (else
      (bind _output_get (set `self.HP` (`KismetMathLibrary.FClamp` (- Amount (`self.HP`)) 0.0 (`self.MaxHP`))))
      (if (== _output_get 0.0)
        (`KismetSystemLibrary.PrintString` "Update Resources")
        (bind _returnvalue_2 (`GameplayStatics.GetActorOfClass` "/Game/Blueprints/BP_GridManager.BP_GridManager_C"))
        (message `/Game/Interface/BPI_Grid.DeadEnemy` _returnvalue_2)
        (`self.K2_DestroyActor`)))))

(fn `Movement`
  (bind (_movementdirection_x _movementdirection_y) (break `IntPoint` (`self.MovementDirection`)))
  (`self.K2_SetActorLocation` (+ (`self.K2_GetActorLocation`) (`KismetMathLibrary.MakeVector` (* _movementdirection_y (`self.MovementSpeed`)) (* _movementdirection_x (`self.MovementSpeed`))))))

(fn `UserConstructionScript`)