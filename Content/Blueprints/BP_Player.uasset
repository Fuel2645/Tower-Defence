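; BP_Player is the player's camera-style pawn and tower placement controller for a grid-based, wave-driven tower defense game.
; Move input pans it within bounds taken from BP_GridManager's grid size, while scroll changes its height within a clamped range.
; When placement is enabled, hovered tiles request a temporary path and Select places a tower through the grid manager.
; Wave and placement state changes refresh the WBP_Tower UI, and starting a wave disables placement.
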(event `self.ReceiveBeginPlay`
  (bind _returnvalue (`GameplayStatics.GetActorOfClass` "/Game/Blueprints/BP_GridManager.BP_GridManager_C"))
  (set `self.MaxX` (* (- (`GridManager.GridHeight` _returnvalue) 1) 100))
  (set `self.MaxY` (* (- (`GridManager.GridWidth` _returnvalue) 1) 100))
  (bind _returnvalue_2 (`|CreateWidget` "/Game/UI/WBP_Tower.WBP_Tower_C"))
  (bind _output_get (set `self.Main UI` _returnvalue_2))
  (`UserWidget.AddToViewport` _output_get 0))

(event `EnhancedInput|/Game/INput/IA_Move`
  (params (ActionValue :type "Vector2D Structure") (ElapsedSeconds :type "Float (double-precision)") (TriggeredSeconds :type "Float (double-precision)") (InputAction :type "InputAction Object Reference" :default "/Game/INput/IA_Move.IA_Move"))
  (bind (_returnvalue_x _returnvalue_y _returnvalue_z) (`KismetMathLibrary.BreakVector` (+ (`self.K2_GetActorLocation`) (`KismetMathLibrary.MakeVector` (* ActionValue_X (`self.Movespeed`)) (* ActionValue_Y (`self.Movespeed`))))))
  (:`Triggered`
    (`self.K2_SetActorLocation` (`KismetMathLibrary.MakeVector` (`KismetMathLibrary.FClamp` _returnvalue_x 0.0 (`self.MaxX`)) (`KismetMathLibrary.FClamp` _returnvalue_y 0.0 (`self.MaxY`)) _returnvalue_z))))

(event `EnhancedInput|/Game/INput/IA_Scroll`
  (params (ActionValue :type "Float (double-precision)") (ElapsedSeconds :type "Float (double-precision)") (TriggeredSeconds :type "Float (double-precision)") (InputAction :type "InputAction Object Reference" :default "/Game/INput/IA_Scroll.IA_Scroll"))
  (bind (_returnvalue_x _returnvalue_y _returnvalue_z) (`KismetMathLibrary.BreakVector` (+ (`self.K2_GetActorLocation`) (`KismetMathLibrary.MakeVector` 0.0 0.0 (* ActionValue (`self.Scroll Speed`))))))
  (:`Triggered`
    (`self.K2_SetActorLocation` (`KismetMathLibrary.MakeVector` _returnvalue_x _returnvalue_y (`KismetMathLibrary.FClamp` _returnvalue_z 200.0 1700.0)))))

(event `/Game/Interface/BPI_Towers.SetHoveredTile`
  (params (`Tile Coord` :type "IntPoint Structure"))
  (set `self.HoveredOverTile` `Tile Coord`)
  (if (`self.CanPlaceTower`)
    (bind _returnvalue (`GameplayStatics.GetActorOfClass` "/Game/Blueprints/BP_GridManager.BP_GridManager_C"))
    (`/Game/Blueprints/BP_GridManager.Temp Path` _returnvalue (`self.HoveredOverTile`))))

(event `EnhancedInput|/Game/INput/IA_Select`
  (params (ActionValue :type Boolean) (ElapsedSeconds :type "Float (double-precision)") (TriggeredSeconds :type "Float (double-precision)") (InputAction :type "InputAction Object Reference" :default "/Game/INput/IA_Select.IA_Select"))
  (:`Started`
    (if (`self.CanPlaceTower`)
      (bind _returnvalue (`GameplayStatics.GetActorOfClass` "/Game/Blueprints/BP_GridManager.BP_GridManager_C"))
      (`/Game/Blueprints/BP_GridManager.Place Tower` _returnvalue (`self.HoveredOverTile`)))))

(event `/Game/Interface/BPI_Player.WaveStart`
  (set `self.WavePlaying` true)
  (set `self.CanPlaceTower` false)
  (`/Game/UI/WBP_Tower.Colour Set` (`self.Main UI`)))

(event `/Game/Interface/BPI_Player.Wave Ended`
  (set `self.WavePlaying` false)
  (`/Game/UI/WBP_Tower.Colour Set` (`self.Main UI`)))

(event `/Game/Interface/BPI_Towers.SetCanPlaceTower`
  (set `self.CanPlaceTower` (not (`self.CanPlaceTower`)))
  (`/Game/UI/WBP_Tower.Colour Set` (`self.Main UI`)))

(fn `GetCanPlaceTower`
  (returns (`can place tower` :type Boolean))
  (return (`self.CanPlaceTower`)))

(fn `GetWaveStatus`
  (returns (Status :type Boolean))
  (return (`self.WavePlaying`)))

(fn `UserConstructionScript`)